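; A callable elevator platform that descends when the player character overlaps its CallElevator trigger, then returns to its start.
; BeginPlay caches the transforms of the Cube platform and the Plane, which marks the bottom stop.
; After delays, a timeline lerps the Cube down, and following a pause a second timeline lerps it back up.
; An IsReady flag blocks new calls until the round trip finishes.
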(event OnComponentBeginOverlap(callelevator)
  (params (OverlappedComponent :type Primitive%20Component%20Object%20Reference) (OtherActor :type Actor%20Object%20Reference) (OtherComp :type Primitive%20Component%20Object%20Reference) (OtherBodyIndex :type Integer) (bFromSweep :type Boolean) (SweepResult :type Hit%20Result%20Structure%20%28by%20ref%29))
  ;[0.15 0.15 0.15 0.5] Comment
  (Development|PrintString "Calling Elevator")
  (if (Variables|Default|GetIs%20Ready)
    (Utilities|Casting|CastToBP_Custom3rdPerChar OtherActor)
    (CallFunction|Activated)))

(event Custom|lowering
  ;[0.15 0.15 0.15 0.5] Comment
  (Development|PrintString "Lowering Platform")
  (Utilities|FlowControl|Delay 2.0)
  (bind _newtrack_0 (Timeline|Timeline_0 PlayFromStart)
    (:Update
      (Transformation|SetWorldLocationAndRotation (Variables|Default|GetCube) (.location (Math|Transform|Lerp(Transform) (Variables|Default|GetPlatformStart) (Variables|Default|Getground) _newtrack_0)) (.rotation (Math|Transform|Lerp(Transform) (Variables|Default|GetPlatformStart) (Variables|Default|Getground) _newtrack_0)) false false))
    (:Finished
      (Development|PrintString "platform ready")
      (Utilities|FlowControl|Delay 5.0)
      (CallFunction|GoingUp))))

(event Custom|activated
  ;[0.15 0.15 0.15 0.5] Comment
  (Development|PrintString "Calling Elevator")
  (Variables|Default|SetIs%20Ready false)
  (Utilities|FlowControl|Delay (Variables|Default|GetFallDelay))
  (CallFunction|Lowering))

(event Custom|GoingUp
  ;[0.15 0.15 0.15 0.5] Comment
  (Development|PrintString "Moving Up")
  (bind _newtrack_0 (Timeline|Timeline PlayFromStart)
    (:Update
      (Transformation|SetWorldLocationAndRotation (Variables|Default|GetCube) (.location (Math|Transform|Lerp(Transform) (Variables|Default|Getground) (Variables|Default|GetPlatformStart) _newtrack_0)) (.rotation (Math|Transform|Lerp(Transform) (Variables|Default|Getground) (Variables|Default|GetPlatformStart) _newtrack_0)) false false))
    (:Finished
      (Variables|Default|SetIs%20Ready true))))

(event EventBeginPlay
  ;[0.15 0.15 0.15 0.5] Comment
  (Variables|Default|SetPlatformStart (Transformation|GetWorldTransform (Variables|Default|GetCube)))
  (Variables|Default|Setground (Transformation|GetWorldTransform (Variables|Default|GetPlane)))
  (Development|PrintString "ElevatorReady"))

(fn ConstructionScript)