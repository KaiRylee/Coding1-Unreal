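; BP_SpawnManager runs wave-based enemy spawning at the BP_SpawnPoint actors placed in the level.
; Shortly after BeginPlay, SpawnEenemies loops over every spawn point and uses a weighted random roll to decide whether each spawns a BP_Enemy.
; NewWaveCheck, meant to be called by dying enemies, counts remaining BP_Enemy actors and respawns a wave after a delay when at most one remains.
; Print strings trace each step.
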(event Custom|Spawn%20Eenemies
  (bind _outactors (Actor|GetAllActorsOfClass "/Game/Blueprints/BP_SpawnPoint.BP_SpawnPoint_C")) ; get array of all spawn points in the level
  (for _array_element _outactors
    (Development|PrintString (Utilities|GetDisplayName _array_element) true true "(R=0.000000,G=0.660000,B=1.000000,A=1.000000)" 1e+01)
    (if (Math|Random|RandomBoolwithWeight 0.8)
      (Game|SpawnActorfromClass "/Game/Blueprints/BP_Enemy.BP_Enemy_C" (Transformation|GetWorldTransform (Variables|/Game/Blueprints/BP_SpawnPoint.BP_SpawnPoint_C|GetDefaultSceneRoot _array_element)) "Undefined" "MultiplyWithRoot" 0 0))))

(event Custom|NewWaveCheck
  (Development|PrintString "Hello")
  (bind _outactors (Actor|GetAllActorsOfClass "/Game/Blueprints/BP_Enemy.BP_Enemy_C"))
  (Development|PrintString (Utilities|String|Append "There are " (Utilities|String|ToString(Integer) (Utilities|Array|Length _outactors))))
  (if (> (Utilities|Array|Length _outactors) 1)
    (Development|PrintString "You are not the last one")
    (else
      (Development|PrintString "NEW WAVE INCOMING" true true "(R=0.781250,G=0.036444,B=0.000000,A=1.000000)")
      (Utilities|FlowControl|Delay 2.0)
      (CallFunction|SpawnEenemies))))

(event EventBeginPlay
  (Development|PrintString "WE ARE HERE - spawn maanger")
  (Utilities|FlowControl|Delay 1.0)
  (CallFunction|SpawnEenemies))

(fn ConstructionScript)